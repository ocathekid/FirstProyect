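; Guard AI pawn that investigates, patrols, chases seen pawns and returns to its starting position.
; Investigate receives a destination and patrol points, moves there, then walks the points in order unless chasing.
; PawnSensing triggers Chase toward the pawn's last seen location, then back to station; only a failed move clears Chasing.
; A BeginPlay delay loop checks player proximity until a catch, which resets the player to checkpoint.
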(event OnSeePawn(PawnSensing)
  (params (Pawn :type Pawn%20Object%20Reference))
  (CallFunction|Chase))

(event Custom|Chase
  (Variables|Default|SetChasing true)
  (AI|AIMoveTo self (Transformation|GetActorLocation (stale OnSeePawn(PawnSensing) Pawn)) 0 5e+01 false
    (:OnSuccess
      (Development|PrintString "we are at the player's last known location"))
    (:OnFail
      (Variables|Default|SetChasing false)))
  (CallFunction|ReturntoGuardStation))

(event Custom|Investigate
  (params (Destination :type Vector) (PatrolPoints :type Array%20of%20Actor%20Object%20References))
  (Variables|Default|SetPatrolPoints PatrolPoints)
  (Variables|Default|SetIndex 0)
  (bind _movementresult (AI|AIMoveTo self Destination 0 1e+02 false)
    (:then
      (switch Utilities|FlowControl|Switch|SwitchonEPathFollowingResult _movementresult
        (:Success
          _)
        (:Blocked
          _)
        (:OffPath
          _)
        (:Invalid
          _))
      (Utilities|FlowControl|RetriggerableDelay 2.0)
      (if (not (Variables|Default|GetChasing))
        (CallFunction|Patrol)))))

(event Custom|Return%20to%20Guard%20Station
  (AI|AIMoveTo self (Variables|Default|GetStart%20Location) 0 1e+02 false))

(event Custom|Patrol
  (AI|AIMoveTo self "0, 0, 0" (Utilities|Array|Get(acopy) (Variables|Default|GetPatrolPoints) (Variables|Default|GetIndex)) 5.0 false :!label _label
    (:OnSuccess
      (Utilities|FlowControl|Delay 2.0)
      (Math|Integer|IncrementInt (Variables|Default|GetIndex)
        (:%20%20
          (if (not (Variables|Default|GetChasing))
            (if (>= (Variables|Default|GetIndex) (Utilities|Array|Length (Variables|Default|GetPatrolPoints)))
              (CallFunction|ReturntoGuardStation)
              (else
                (goto _label)))))))))

(event EventBeginPlay
  (Variables|Default|SetStart%20Location (Transformation|GetWorldLocation (Variables|Collision|GetCapsuleComponent)))
  (if (<= (Math|Vector|Distance(Vector) (Transformation|GetWorldLocation (Variables|Collision|GetCapsuleComponent)) (Transformation|GetWorldLocation (Variables|/Script/Engine.Character|GetCapsuleComponent (Game|GetPlayerCharacter 0)))) 1e+02) :!label _label
    (Development|PrintString "You died")
    (bind _asbp_first_person_character (Utilities|Casting|CastToBP_FirstPersonCharacter (Game|GetPlayerCharacter 0)))
    (Default|ResettoCheckpoint _asbp_first_person_character)
    (else
      (Utilities|FlowControl|Delay 0.2)
      (goto _label))))

(fn ConstructionScript)