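; Security camera Blueprint that detects the first-person player through AI Perception and alerts guards.
; On sensing, it waits briefly, re-tests the same event stimulus, then switches the cube to a detected material.
; It then sends every guard sharing its GroupID to investigate the player's position, passing along its patrol point.
; On losing the player it spawns a Shadow actor at the player's current location.
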(event OnComponentActivated(AIPerception)
  (params (Component :type Actor%20Component%20Object%20Reference) (bReset :type Boolean))
  (Development|PrintString "Activated"))

(event OnTargetPerceptionUpdated(AIPerception)
  (params (Actor :type Actor%20Object%20Reference) (Stimulus :type AI%20Stimulus%20Structure))
  (bind _bsuccessfullysensed (Utilities|Struct|BreakAIStimulus Stimulus))
  (bind _asbp_first_person_character (Utilities|Casting|CastToBP_FirstPersonCharacter Actor))
  (if _bsuccessfullysensed
    (Development|PrintString "I see you")
    (Utilities|FlowControl|Delay 2.0)
    (if _bsuccessfullysensed
      (Rendering|Material|SetMaterialbyName (Variables|Default|GetCube) "None" "/Game/GuardLevel/Materials/M_detected.M_detected")
      (Development|PrintString "Calling Guards" true true "(R=1.000000,G=0.030315,B=0.013735,A=1.000000)")
      (bind _outactors (Actor|GetAllActorsOfClass "/Game/GuardLevel/BP/BP_Guard_AI.BP_Guard_AI_C"))
      (for _array_element _outactors
        (if (== (Variables|Default|GetGroupID) (Variables|/Game/GuardLevel/BP/BP_Guard_AI.BP_Guard_AI_C|GetGroupID _array_element))
          (Default|Investigate _array_element (Transformation|GetWorldLocation (Variables|/Script/Engine.Character|GetCapsuleComponent _asbp_first_person_character)) (Variables|Default|GetPatrolPoint)))))
    (else
      (Development|PrintString "I can't see you")
      (Game|SpawnActorfromClass "/Game/ThirdPerson/Blueprints/Shadow.Shadow_C" (Math|Transform|MakeTransform (Transformation|GetWorldLocation (Variables|/Script/Engine.Character|GetCapsuleComponent _asbp_first_person_character)) (Math|Conversions|RotationFromXVector (Transformation|GetWorldLocation (Variables|/Script/Engine.Character|GetCapsuleComponent _asbp_first_person_character))) "1.000000,1.000000,1.000000") "Undefined" "MultiplyWithRoot" 0 0))))

(fn ConstructionScript)